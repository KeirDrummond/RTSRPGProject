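; Game mode Blueprint that shows the winner screen when a match ends.
; Its EndGame event calls the parent, then reads the Alive flag on player controller 0's GamePlayerState.
; It picks the first PlayerArray entry as winner if that player is alive, otherwise the second, assuming a two-player order.
; It then creates an EndGameMenu widget for that controller, passes it the winner and adds it to the viewport.
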(event `self.EndGame`
  (bind _returnvalue (`GameplayStatics.GetPlayerController` 0))
  (bind _playerarray (`GameStateBase.PlayerArray` (`GameplayStatics.GetGameState`)))
  (`parent.EndGame`)
  (bind _asgame_player_state (cast `GamePlayerState` (`Controller.PlayerState` _returnvalue)))
  (if (`GamePlayerState.alive` _asgame_player_state)
    (set `self.Winner` (`|GetArrayItem` _playerarray))
    (else
      (set `self.Winner` (`|GetArrayItem` _playerarray 1))))
  (bind _returnvalue_2 (`|GenericCreateObject` "/Game/UserInterface/EndGameMenu.EndGameMenu_C" _returnvalue))
  (`/Game/UserInterface/EndGameMenu.Set Winner` _returnvalue_2 (`self.Winner`))
  (`UserWidget.AddToViewport` _returnvalue_2 0))

(fn `UserConstructionScript`)